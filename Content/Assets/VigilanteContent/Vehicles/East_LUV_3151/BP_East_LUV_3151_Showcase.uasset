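; Showcase Blueprint for the East LUV 3151 vehicle, exposing its appearance and moving parts to showcase controls.
; Generic button, checkbox and slider events forward their values to named setters for skin, damage, wheels, wipers, mirrors, front light holder and light emissivity.
; A twin slider uses a first-slider flag to drive either front or back door angle.
; The construction script only calls its parent.
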(event `/Game/Assets/VigilanteContent/Shared/Blueprints/Showcase/Interfaces/BP_ShowcaseControlsInterface.SetButtonsVariable0`
  (params (NewIndex :type Integer))
  ;[1 1 1] Set Skyn Type
  (`self.SetSkinType` (`KismetMathLibrary.Conv_IntToDouble` NewIndex)))

(event `/Game/Assets/VigilanteContent/Shared/Blueprints/Showcase/Interfaces/BP_ShowcaseControlsInterface.SetCheckboxVariable0`
  (params (NewState :type Boolean))
  ;[1 1 1] Showcase checkbox controls
  (`self.SetShowDamaged` NewState))

(event `/Game/Assets/VigilanteContent/Shared/Blueprints/Showcase/Interfaces/BP_ShowcaseControlsInterface.SetSliderVariable0`
  (params (NewValue :type "Float (double-precision)"))
  ;[1 1 1] Showcase float controls
  (`self.SetWheelSpeed` NewValue))

(event `/Game/Assets/VigilanteContent/Shared/Blueprints/Showcase/Interfaces/BP_ShowcaseControlsInterface.SetSliderVariable1`
  (params (NewValue :type "Float (double-precision)"))
  ;[1 1 1] Showcase float controls
  (`self.SetWheelAngle` NewValue))

(event `/Game/Assets/VigilanteContent/Shared/Blueprints/Showcase/Interfaces/BP_ShowcaseControlsInterface.SetSliderVariable2`
  (params (NewValue :type "Float (double-precision)"))
  ;[1 1 1] Showcase float controls
  (`self.SetWindowCleanersAngle` NewValue))

(event `/Game/Assets/VigilanteContent/Shared/Blueprints/Showcase/Interfaces/BP_ShowcaseControlsInterface.SetSliderVariable3`
  (params (NewValue :type "Float (double-precision)"))
  ;[1 1 1] Showcase float controls
  (`self.SetMirrorsAngle` NewValue))

(event `/Game/Assets/VigilanteContent/Shared/Blueprints/Showcase/Interfaces/BP_ShowcaseControlsInterface.SetSliderVariable4`
  (params (NewValue :type "Float (double-precision)"))
  ;[1 1 1] Showcase float controls
  (`self.Set FrontLightHolderAngle` NewValue))

(event `/Game/Assets/VigilanteContent/Shared/Blueprints/Showcase/Interfaces/BP_ShowcaseControlsInterface.SetSliderVariable5`
  (params (NewValue :type "Float (double-precision)"))
  ;[1 1 1] Showcase float controls
  (`self.SetLightsEmissivity` NewValue))

(event `/Game/Assets/VigilanteContent/Shared/Blueprints/Showcase/Interfaces/BP_ShowcaseControlsInterface.SetTwinSliderVariable0`
  (params (`bFirstSlider?` :type Boolean) (NewFirstValue :type "Float (double-precision)") (NewSecondValue :type "Float (double-precision)"))
  ;[1 1 1] Showcase float controls
  (if `bFirstSlider?`
    (`self.SetFrontDoorsAngle` NewFirstValue)
    (else
      (`self.SetBackDoorsAngle` NewSecondValue))))

(fn `UserConstructionScript`
  (`parent.UserConstructionScript`))