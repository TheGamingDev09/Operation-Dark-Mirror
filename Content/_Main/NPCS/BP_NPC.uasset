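; BP_NPC is an armed enemy that chases the player, fires projectiles and awards score when hit.
; Pawn sensing flags detection, starts a repeating AIMoveTo chase and fires from the attached BP_M4's muzzle.
; Per-body-part hitboxes set damage multipliers and point bonuses, doubling points while the player is undetected.
; At zero health it destroys itself and its weapon, then drops a random health or ammo pickup.
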(event `self.ReceiveAnyDamage`
  (params (Damage :type "Float (single-precision)") (DamageType :type "DamageType Object Reference") (InstigatedBy :type "Controller Object Reference") (DamageCauser :type "Actor Object Reference"))
  (bind _returnvalue (`self.K2_GetActorLocation`))
  ;[1 1 1] Damage System
  (set `self.health` (`KismetMathLibrary.FClamp` (- (`self.health`) Damage) 0.0 (`self.MaxHealth`)))
  ;[1 1 1] Damage and Score
  (if (<= (`self.health`) 0.0)
    (`self.K2_DestroyActor` self :!label _label)
    (`self.K2_DestroyActor` (`self.M4Ref`))
    (set `self.RandomNumber` (`KismetMathLibrary.RandomInteger` 2))
    (if (== (`self.RandomNumber`) 1)
      (`|SpawnActorFromClass` "/Game/FirstPerson/Blueprints/BP_Health_PickUp.BP_Health_PickUp_C" (`KismetMathLibrary.MakeTransform` _returnvalue) "Undefined" "MultiplyWithRoot" null null)
      (else
        (`|SpawnActorFromClass` "/Game/FirstPerson/Blueprints/BP_Ammo_Pickup.BP_Ammo_Pickup_C" (`KismetMathLibrary.MakeTransform` _returnvalue) "Undefined" "MultiplyWithRoot" null null)))))

(event `self.ReceiveTick`
  (params (DeltaSeconds :type "Float (single-precision)"))
  ;[1 1 1] Damage and Score
  (if (<= (`self.health`) 0.0)
    (goto _label)))

(event `self.HeadHitbox.OnComponentHit`
  (params (HitComponent :type "PrimitiveComponent Object Reference") (OtherActor :type "Actor Object Reference") (OtherComp :type "PrimitiveComponent Object Reference") (NormalImpulse :type "Vector Structure") (Hit :type "HitResult Structure (by ref)"))
  (bind _returnvalue (* 5 (`self.PointBonus`)))
  ;[1 1 1] Damage and Score
  (set `self.PointBonus` 0)
  (set `self.DamageMultiplier` 2.0)
  (`GameplayStatics.ApplyDamage` self (* (`self.Base Damage`) (`self.DamageMultiplier`)) :!label _label_2)
  (bind _asbp_first_person_character (cast `/Game/FirstPerson/Blueprints/BP_FirstPersonCharacter` (`GameplayStatics.GetPlayerCharacter` 0)))
  (if (`self.detected`)
    (set `/Game/FirstPerson/Blueprints/BP_FirstPersonCharacter.Score` (+ (`/Game/FirstPerson/Blueprints/BP_FirstPersonCharacter.Score` _asbp_first_person_character) _returnvalue) _asbp_first_person_character)
    (else
      (set `/Game/FirstPerson/Blueprints/BP_FirstPersonCharacter.Score` (+ (`/Game/FirstPerson/Blueprints/BP_FirstPersonCharacter.Score` _asbp_first_person_character) (* _returnvalue 2)) _asbp_first_person_character))))

(event `self.ChestHitbox.OnComponentHit`
  (params (HitComponent :type "PrimitiveComponent Object Reference") (OtherActor :type "Actor Object Reference") (OtherComp :type "PrimitiveComponent Object Reference") (NormalImpulse :type "Vector Structure") (Hit :type "HitResult Structure (by ref)"))
  ;[1 1 1] Damage and Score
  (set `self.PointBonus` 10)
  (set `self.DamageMultiplier` 1.0 :!label _label_3)
  (goto _label_2))

(event `self.LowerChestHitbox.OnComponentHit`
  (params (HitComponent :type "PrimitiveComponent Object Reference") (OtherActor :type "Actor Object Reference") (OtherComp :type "PrimitiveComponent Object Reference") (NormalImpulse :type "Vector Structure") (Hit :type "HitResult Structure (by ref)"))
  ;[1 1 1] Damage and Score
  (set `self.PointBonus` 5)
  (goto _label_3))

(event `self.RightArmHitBox.OnComponentHit`
  (params (HitComponent :type "PrimitiveComponent Object Reference") (OtherActor :type "Actor Object Reference") (OtherComp :type "PrimitiveComponent Object Reference") (NormalImpulse :type "Vector Structure") (Hit :type "HitResult Structure (by ref)"))
  ;[1 1 1] Damage and Score
  (set `self.PointBonus` 1 :!label _label_4)
  (set `self.DamageMultiplier` 0.5 :!label _label_5)
  (goto _label_2))

(event `self.LeftArmHitBox.OnComponentHit`
  (params (HitComponent :type "PrimitiveComponent Object Reference") (OtherActor :type "Actor Object Reference") (OtherComp :type "PrimitiveComponent Object Reference") (NormalImpulse :type "Vector Structure") (Hit :type "HitResult Structure (by ref)"))
  ;[1 1 1] Damage and Score
  (goto _label_4))

(event `self.LowerLeftArmHitBox.OnComponentHit`
  (params (HitComponent :type "PrimitiveComponent Object Reference") (OtherActor :type "Actor Object Reference") (OtherComp :type "PrimitiveComponent Object Reference") (NormalImpulse :type "Vector Structure") (Hit :type "HitResult Structure (by ref)"))
  ;[1 1 1] Damage and Score
  (goto _label_4))

(event `self.LowerRightArmHitBox.OnComponentHit`
  (params (HitComponent :type "PrimitiveComponent Object Reference") (OtherActor :type "Actor Object Reference") (OtherComp :type "PrimitiveComponent Object Reference") (NormalImpulse :type "Vector Structure") (Hit :type "HitResult Structure (by ref)"))
  ;[1 1 1] Damage and Score
  (goto _label_4))

(event `self.LegHitbox.OnComponentHit`
  (params (HitComponent :type "PrimitiveComponent Object Reference") (OtherActor :type "Actor Object Reference") (OtherComp :type "PrimitiveComponent Object Reference") (NormalImpulse :type "Vector Structure") (Hit :type "HitResult Structure (by ref)"))
  ;[1 1 1] Damage and Score
  (set `self.PointBonus` 2)
  (goto _label_5))

(event `self.ReceiveBeginPlay`
  ;[1 1 1] AI
  (`|ExecutionSequence`
    (:`then_0`
      (bind _returnvalue (`|SpawnActorFromClass` "/Game/FirstPerson/Blueprints/BP_M4.BP_M4_C" (`KismetMathLibrary.MakeTransform` (0.0 0.0 0.0)) "Undefined" "MultiplyWithRoot" null null))
      (bind _output_get (set `self.M4Ref` _returnvalue))
      (`self.K2_AttachToComponent` _output_get (`self.Mesh`) "middle_01_r" "SnapToTarget" "SnapToTarget" "SnapToTarget" true))))

(event `MoveNPC`
  ;[1 1 1] AI
  (`|AIMoveTo` self (0.0 0.0 0.0) (`GameplayStatics.GetPlayerCharacter` 0) 10.0
    (:`OnSuccess`
      (`KismetSystemLibrary.Delay` 1.0))
    (:`OnFail`
      (`KismetSystemLibrary.Delay` 1.0)))
  (`self.MoveNPC`))

(event `self.PawnSensing.OnSeePawn`
  (params (Pawn :type "Pawn Object Reference"))
  ;[1 1 1] AI
  (set `self.detected` true)
  (`self.MoveNPC`)
  (`KismetSystemLibrary.Delay` 0.2)
  (`self.Fire`))

(event `Fire`
  ;[1 1 1] AI
  (`self.K2_SetActorRotation` (`GameplayStatics.GetPlayerCharacter` 0) (`KismetMathLibrary.MakeRotator` 0.0) false)
  (`KismetSystemLibrary.Delay` 0.2)
  (`|SpawnActorFromClass` "/Game/FirstPerson/Blueprints/BP_FirstPersonProjectile.BP_FirstPersonProjectile_C" (`KismetMathLibrary.MakeTransform` (+ (`SceneComponent.K2_GetComponentLocation` (`/Game/FirstPerson/Blueprints/BP_M4.Muzzle` (`self.M4Ref`))) (`KismetMathLibrary.GreaterGreater_VectorRotator` (`self.ProjectileOffset`))) (`self.GetControlRotation`)) "Undefined" "MultiplyWithRoot" null null))

(fn `UserConstructionScript`)